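; BP_Water is a water volume actor with a configurable surface material and underwater post-process look.
; The construction script tints the post process, optionally from the surface color, and feeds a dynamic material instance, tiled by actor scale.
; CoralMacro, not called in the graphs shown, scatters coral meshes via random downward traces within the box, filtered by depth, optionally retrying misses, scaling count with area size and aligning to normals.
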(fn `UserConstructionScript`
  (bind _watermaterial (`self.WaterMaterial`))
  (bind _underwatercolor (`self.UnderwaterColor`))
  (bind _gamma (`self.Gamma`))
  ;[0 0 0] Setting texture parameters and Post Process
  (`PrimitiveComponent.SetMaterial` (`self.WaterMesh`) 0 (`self.Material`))
  (if (`self.UseSurfaceColor`)
    (set `self.UnderwaterColor` (`self.Overall Color`)))
  (setmembers `PostProcessSettings` :`StructRef` (`PostProcessComponent.Settings` (`self.PostProcess`)) :`ColorGamma` (`KismetMathLibrary.MakeVector4` _gamma _gamma _gamma 1.0) :`FilmWhitePoint` _underwatercolor :`SceneColorTint` _underwatercolor :`SceneFringeIntensity` (`self.Fringe`) :`BloomIntensity` (`self.Bloom Intensity`) :`BloomThreshold` (`self.Bloom Threshold`) :`VignetteIntensity` (`self.VignetteIntensity`))
  (bind _returnvalue (`PrimitiveComponent.CreateDynamicMaterialInstance` (`self.WaterMesh`) 0 null "None"))
  (set `self.WaterMaterial` _returnvalue)
  (`MaterialInstanceDynamic.SetScalarParameterValue` _watermaterial "TilingU" (.x (`self.GetActorScale3D`)))
  (`MaterialInstanceDynamic.SetScalarParameterValue` _watermaterial "Tilingv" (.y (`self.GetActorScale3D`)))
  (`MaterialInstanceDynamic.SetScalarParameterValue` _watermaterial "Tiling" (`self.Tiling`))
  (`MaterialInstanceDynamic.SetScalarParameterValue` _watermaterial "WaterOpacity" (`self.Opacity`))
  (`MaterialInstanceDynamic.SetScalarParameterValue` _watermaterial "FadeDistance" (`self.FadeDistance`))
  (`MaterialInstanceDynamic.SetScalarParameterValue` _watermaterial "Metallic" (`self.Metallic`))
  (`MaterialInstanceDynamic.SetScalarParameterValue` _watermaterial "Roughness" (`self.Roughness`))
  (`MaterialInstanceDynamic.SetScalarParameterValue` _watermaterial "RippleSpeed" (`self.RippleSpeed`))
  (`MaterialInstanceDynamic.SetScalarParameterValue` _watermaterial "ExpotentIn" (`self.ExpotentIn`))
  (`MaterialInstanceDynamic.SetScalarParameterValue` _watermaterial "BaseReflectIn" (`self.BaseReflectIn`))
  (`MaterialInstanceDynamic.SetScalarParameterValue` _watermaterial "RefractionWarp" (`self.RefractionWarp`))
  (`MaterialInstanceDynamic.SetScalarParameterValue` _watermaterial "RefractionExponentIn" (`self.RefractionExp`))
  (`MaterialInstanceDynamic.SetScalarParameterValue` _watermaterial "WaveHeight" (`self.WaveHeight`))
  (`MaterialInstanceDynamic.SetVectorParameterValue` _watermaterial "Color" (`self.Overall Color`))
  (`MaterialInstanceDynamic.SetVectorParameterValue` _watermaterial "FresnelColor1" (`self.FresnelColor1`))
  (`MaterialInstanceDynamic.SetVectorParameterValue` _watermaterial "FresnelColor2" (`self.FresnelColor2`))
  (`MaterialInstanceDynamic.SetTextureParameterValue` _watermaterial "RippleNormal" (`self.Ripple Normal`))
  (`MaterialInstanceDynamic.SetTextureParameterValue` _watermaterial "ReflectionTexture" (`self.ReflectionVector`)))