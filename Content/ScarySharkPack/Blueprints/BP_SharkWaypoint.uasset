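; BP_SharkWaypoint is an actor that swims an animated shark mesh in an endless loop along its spline.
; BeginPlay starts the looping graceful swim animation on the skeletal mesh.
; Each Tick places the mesh at the current spline distance in local space, with a yaw offset to correct its facing.
; Distance advances by Speed per frame, unscaled by delta time, and resets to zero at the spline's end.
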(event `self.ReceiveTick`
  (params (DeltaSeconds :type "Float (single-precision)"))
  ;[0 0 0] Set location and rotation per tick
  (`SceneComponent.K2_SetRelativeLocationAndRotation` (`self.SkeletalMesh`) (.location (`SplineComponent.GetTransformAtDistanceAlongSpline` (`self.Spline`) (`self.Distance`) "Local" false)) (`KismetMathLibrary.MakeRotator` (.roll (.rotation (`SplineComponent.GetTransformAtDistanceAlongSpline` (`self.Spline`) (`self.Distance`) "Local" false))) (.pitch (.rotation (`SplineComponent.GetTransformAtDistanceAlongSpline` (`self.Spline`) (`self.Distance`) "Local" false))) (+ (.yaw (.rotation (`SplineComponent.GetTransformAtDistanceAlongSpline` (`self.Spline`) (`self.Distance`) "Local" false))) -90.0)) false false)
  ;[0 0 0] Add next distance calculation
  (set `self.Distance` (+ (`self.Distance`) (`self.Speed`)))
  ;[0 0 0] Check if Distance is more than spline length
  (`/Engine/EditorBlueprintResources/StandardMacros.CompareFloat` (`self.Distance`) (`SplineComponent.GetSplineLength` (`self.Spline`))
    (:`>`
      _)
    (:`==`
      _))
  ;[0 0 0] Loop at 0 distance
  (set `self.Distance` 0.0))

(event `self.ReceiveBeginPlay`
  ;[0 0 0] Play looped Shark Animation
  (`SkeletalMeshComponent.PlayAnimation` (`self.SkeletalMesh`) "/Game/ScarySharkPack/Character/Animations/A_Shark_GracefulSwim.A_Shark_GracefulSwim" true))

(fn `UserConstructionScript`)