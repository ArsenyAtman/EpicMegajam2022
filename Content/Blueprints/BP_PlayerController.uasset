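; BP_PlayerController lets two local players each steer a BP_Ship through one player controller.
; On BeginPlay the first controller caches another BP_Ship as the second pawn, while any other controller disables its input.
; P1 inputs drive the possessed ship and _P2 inputs drive the cached one.
; Stored axis values feed Move, and action presses call Fire and Dive.
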(event `self.ReceiveBeginPlay`
  (if (== (`GameplayStatics.GetPlayerController` 0) self)
    (bind _outactors (`GameplayStatics.GetAllActorsOfClass` "/Game/Blueprints/BP_Ship.BP_Ship_C"))
    (for _array_element _outactors
      (if (!= _array_element (`self.K2_GetPawn`))
        (set `self.SecondControlledPawn` _array_element)
        (break)))
    (else
      (`self.DisableInput` self))))

(event `InputAxis|UpAndDown_P2`
  (params (AxisValue :type "Float (single-precision)"))
  ;[1 1 1] P2
  (set `self.InputX_P2` AxisValue)
  (`/Game/Blueprints/BP_Ship.Move` (cast `/Game/Blueprints/BP_Ship` (`self.SecondControlledPawn`) :!pure true) (`KismetMathLibrary.MakeVector` (`self.InputX_P2`) (`self.InputY_P2`)) :!label _label))

(event `InputAxis|UpAndDown`
  (params (AxisValue :type "Float (single-precision)"))
  ;[1 1 1] P1
  (set `self.InputX` AxisValue)
  (`/Game/Blueprints/BP_Ship.Move` (cast `/Game/Blueprints/BP_Ship` (`self.K2_GetPawn`) :!pure true) (`KismetMathLibrary.MakeVector` (`self.InputX`) (`self.InputY`)) :!label _label_2))

(event `InputAxis|LeftAndRight_P2`
  (params (AxisValue :type "Float (single-precision)"))
  ;[1 1 1] P2
  (set `self.InputY_P2` AxisValue)
  (goto _label))

(event `InputAxis|LeftAndRight`
  (params (AxisValue :type "Float (single-precision)"))
  ;[1 1 1] P1
  (set `self.InputY` AxisValue)
  (goto _label_2))

(event `InputAction|Fire_P2`
  (params (Key :type "Key Structure"))
  ;[1 1 1] P2
  (:`Pressed`
    (`/Game/Blueprints/BP_Ship.Fire` (cast `/Game/Blueprints/BP_Ship` (`self.SecondControlledPawn`) :!pure true))))

(event `InputAction|Fire`
  (params (Key :type "Key Structure"))
  ;[1 1 1] P1
  (:`Pressed`
    (`/Game/Blueprints/BP_Ship.Fire` (cast `/Game/Blueprints/BP_Ship` (`self.K2_GetPawn`) :!pure true))))

(event `InputAction|Dive_P2`
  (params (Key :type "Key Structure"))
  ;[1 1 1] P2
  (:`Pressed`
    (`/Game/Blueprints/BP_Ship.Dive` (cast `/Game/Blueprints/BP_Ship` (`self.SecondControlledPawn`) :!pure true))))

(event `InputAction|Dive`
  (params (Key :type "Key Structure"))
  ;[1 1 1] P1
  (:`Pressed`
    (`/Game/Blueprints/BP_Ship.Dive` (cast `/Game/Blueprints/BP_Ship` (`self.K2_GetPawn`) :!pure true))))

(fn `UserConstructionScript`)