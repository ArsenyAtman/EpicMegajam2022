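; Player ship that sails toward camera-corrected input, fires its child-actor cannons and can toggle diving.
; Tick integrates acceleration and speed-scaled turning into a swept move, while looping timelines bob the hull and drive dive depth and emissive.
; A one-second timer damages it when overlapping ships, landscape or static meshes.
; Damage drives a material parameter; death requests a GameMode respawn, swaps in a wreck mesh, clears cannons and sinks it unless underwater.
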(event `Fire`
  (for _array_element (`self.K2_GetComponentsByClass` "/Script/Engine.ChildActorComponent")
    (bind _asbp_cannon (cast `/Game/Blueprints/BP_Cannon` (`ChildActorComponent.ChildActor` _array_element)))
    (`/Game/Blueprints/BP_Cannon.Fire` _asbp_cannon)))

(event `Move`
  (params (InputVector :type "Vector Structure"))
  (if (> (`self.Health`) 0.0)
    (set `self.InputVector` (`KismetMathLibrary.GreaterGreater_VectorRotator` (`KismetMathLibrary.Normal` InputVector) (`self.CameraCorrection`)))
    (else
      (set `self.InputVector` (0.0 0.0 0.0)))))

(event `self.ReceiveTick`
  (params (DeltaSeconds :type "Float (single-precision)"))
  (bind _maxturnspeed (`self.MaxTurnSpeed`))
  (bind _movementdirection (`self.GetMovementDirection` (`self.InputVector`) (`self.GetActorForwardVector`) (`self.GetActorRightVector`)))
  (set `self.DeltaSeconds` DeltaSeconds)
  (`|ExecutionSequence`
    (:`then_0`
      (set `self.MovementCurrentSpeed` (`KismetMathLibrary.FClamp` (+ (`self.MovementCurrentSpeed`) (* (`KismetMathLibrary.SelectFloat` 1.0 -1.0 (!= (`self.InputVector`) (0.0 0.0 0.0) :`ErrorTolerance` 0.1)) (`self.MovementAcceleration`) (`self.DeltaSeconds`))) 0.0 (`self.MovementMaxSpeed`)))
      (set `self.MovementVelocity` (* (`self.GetActorForwardVector`) (`self.MovementCurrentSpeed`)))
      (if (!= (`self.InputVector`) (0.0 0.0 0.0) :`ErrorTolerance` 0.1)
        (set `self.RotationVelocity` (`KismetMathLibrary.MakeRotator` 0.0 0.0 (`KismetMathLibrary.SelectFloat` (`KismetMathLibrary.FClamp` (* (/ (`self.MovementCurrentSpeed`) (`self.MovementMaxSpeed`)) (`self.RotationCoefficient`) _movementdirection) (* _maxturnspeed -1.0) _maxturnspeed) 0.0 (> (`KismetMathLibrary.Abs` _movementdirection) 1.0))))
        (else
          (set `self.RotationVelocity` (struct)))))
    (:`then_1`
      (`self.K2_SetActorLocationAndRotation` (+ (* (`self.MovementVelocity`) DeltaSeconds) (`self.K2_GetActorLocation`)) (`KismetMathLibrary.ComposeRotators` (* (`self.RotationVelocity`) DeltaSeconds) (`self.K2_GetActorRotation`)) true))))

(event `self.ReceiveBeginPlay`
  (`|ExecutionSequence`
    (:`then_0`
      (bind (_direction _verticalfloating _rollfloating _pitchfloating) (`Timeline|ShipFloating` :`NewTime` (`KismetMathLibrary.RandomFloatInRange` 0.0 30.0) :!via `SetNewTime` :!label _label)
        (:`Update`
          (`SceneComponent.K2_SetRelativeLocation` (`self.ShipBody`) (`KismetMathLibrary.MakeVector` 0.0 0.0 _verticalfloating) true false)
          (`SceneComponent.K2_SetRelativeRotation` (`self.ShipBody`) (* (`KismetMathLibrary.MakeRotator` _rollfloating _pitchfloating) (`self.FloatingCoefficient`)) false false))
        (:`Finished`
          (goto _label :!via `PlayFromStart`))))
    (:`then_1`
      (goto _label))
    (:`then_2`
      (`KismetSystemLibrary.K2_SetTimerDelegate` (delegate `Check collisions`) 1.0 true))))

(event `Check collisions`
  (for _array_element (`PrimitiveComponent.GetOverlappingActors` (`self.Capsule`) null)
    (if (!= _array_element self)
      (cast `/Game/Blueprints/BP_Ship` _array_element
        (:`then`
          _)
        (:`CastFailed`
          (cast `Landscape` _array_element
            (:`then`
              _)
            (:`CastFailed`
              (cast `StaticMeshActor` _array_element)))
          (set `self.IsUnderwater` true)))
      (`GameplayStatics.ApplyDamage` self 200.0 null self))))

(event `Dive`
  (if (not (`self.IsDiving`))
    (set `self.IsDiving` true)
    (bind _isa (`/Engine/EditorBlueprintResources/StandardMacros.FlipFlop`)
      (:`A`
        (set `self.IsUnderwater` _isa)
        (bind (_direction _depth _emissive _rotationcoefficient) (`Timeline|Diving` :!via `PlayFromStart` :!label _label_2)
          (:`Update`
            (`SceneComponent.K2_SetRelativeLocation` (`self.FloatingDeep`) _depth true false)
            (`MaterialInstanceDynamic.SetScalarParameterValue` (`self.MaterialInstance`) "Emissive" _emissive)
            (set `self.FloatingCoefficient` _rotationcoefficient))
          (:`Finished`
            (set `self.IsDiving` false))))
      (:`B`
        (goto _label_2 :!via `ReverseFromEnd`)))))

(event `self.ReceiveAnyDamage`
  (params (Damage :type "Float (single-precision)") (DamageType :type "DamageType Object Reference") (InstigatedBy :type "Controller Object Reference") (DamageCauser :type "Actor Object Reference"))
  (if (> (`self.Health`) 0.0)
    (bind _output_get (set `self.Health` (`KismetMathLibrary.FClamp` (- (`self.Health`) Damage) 0.0 (`self.MaxHealth`))))
    (`|ExecutionSequence`
      (:`then_0`
        (`MaterialInstanceDynamic.SetScalarParameterValue` (`self.MaterialInstance`) "DamageHeightPower" (/ (`self.Health`) (`self.MaxHealth`))))
      (:`then_1`
        (if (<= _output_get 0.0)
          (bind _asbp_game_mode (cast `/Game/Blueprints/BP_GameMode` (`GameplayStatics.GetGameMode`)))
          (`/Game/Blueprints/BP_GameMode.RespawnPlayer` _asbp_game_mode self)
          (set `self.InputVector` (0.0 0.0 0.0))
          (`self.OnDead`)
          (`StaticMeshComponent.SetStaticMesh` (`self.ShipBody`) "/Game/PirateIsland/Frag/SM_broken_ship.SM_broken_ship")
          (`SceneComponent.SetVisibility` (`self.Sails`) false true)
          (for _array_element (`self.K2_GetComponentsByClass` "/Script/Engine.ChildActorComponent")
            (`ChildActorComponent.SetChildActorClass` _array_element null))
          (`GameplayStatics.SpawnSoundAtLocation` "/Game/Sounds/Breaking/SC_Breaking.SC_Breaking" (`SceneComponent.K2_GetComponentLocation` (`self.FloatingDeep`)) (struct) 1.0 1.0 0.0 null null)
          (if (not (`self.IsUnderwater`))
            (bind (_direction _depth) (`Timeline|GoingDown`)
              (:`Update`
                (`SceneComponent.K2_SetRelativeLocation` (`self.FloatingDeep`) _depth true false)))))))))

(fn `DrawDebugVectors`
  (bind _returnvalue (`self.K2_GetActorLocation`))
  (bind _returnvalue_2 (`self.K2_GetActorLocation`))
  (`KismetSystemLibrary.DrawDebugArrow` _returnvalue (+ _returnvalue (* (`self.GetActorForwardVector`) 100.0)) 0.0 (struct :`R` 1.0 :`A` 1.0) 0.0 3.0)
  (`KismetSystemLibrary.DrawDebugArrow` _returnvalue_2 (+ _returnvalue_2 (* (`self.InputVector`) 100.0)) 0.0 (struct :`R` 0.060696 :`G` 1.0 :`A` 1.0) 0.0 3.0))

(fn `GetMovementDirection`
  (params (InputVector :type "Vector Structure") (ActorForwardVector :type "Vector Structure") (ActorRightVector :type "Vector Structure"))
  (returns (MovementDirection :type "Float (double-precision)"))
  (bind _returnvalue (`KismetMathLibrary.SignOfFloat` (`KismetMathLibrary.Dot_VectorVector` InputVector ActorRightVector)))
  (return (`KismetMathLibrary.SelectFloat` 180.0 (* (`KismetMathLibrary.DegAcos` (`KismetMathLibrary.Dot_VectorVector` InputVector ActorForwardVector)) _returnvalue) (and (== _returnvalue 0.0) (!= InputVector ActorForwardVector :`ErrorTolerance` 10.0)))))

(fn `UserConstructionScript`
  (bind (_cameracorrection_roll _cameracorrection_pitch _cameracorrection_yaw) (`KismetMathLibrary.BreakRotator` (`self.CameraCorrection`)))
  (bind _springarm (`self.SpringArm`))
  (bind (_relativerotation_roll _relativerotation_pitch) (`KismetMathLibrary.BreakRotator` (`SceneComponent.RelativeRotation` _springarm)))
  (`SceneComponent.K2_SetRelativeRotation` _springarm (`KismetMathLibrary.MakeRotator` _relativerotation_roll _relativerotation_pitch _cameracorrection_yaw) false false)
  (bind _returnvalue (`PrimitiveComponent.CreateDynamicMaterialInstance` (`self.ShipBody`) 0 "/Game/PirateIsland/Materials/Props/MI_BigShip01_Painted01.MI_BigShip01_Painted01" "None"))
  (set `self.MaterialInstance` _returnvalue))