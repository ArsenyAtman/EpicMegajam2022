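; BP_CannonBall is a cannonball projectile that deals point damage to whatever stops it, then destroys itself.
; On BeginPlay it randomizes its spin rate, reuses that value as the starting rotation, and points both ProjectileMovement and RotatingMovement at the static mesh.
; When the projectile stops, it applies its Damage to the hit actor and spawns a fire gib particle effect only if that actor is a BP_Ship.
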(event `self.ReceiveBeginPlay`
  (bind _output_get (set `RotatingMovementComponent.RotationRate` (`KismetMathLibrary.MakeRotator` (`KismetMathLibrary.RandomFloatInRange` 10.0 90.0) (`KismetMathLibrary.RandomFloatInRange` 10.0 90.0) (`KismetMathLibrary.RandomFloatInRange` 10.0 90.0)) (`self.RotatingMovement`)))
  (`self.K2_SetActorRotation` self _output_get false)
  (`MovementComponent.SetUpdatedComponent` (`self.ProjectileMovement`) (`self.StaticMesh`))
  (`MovementComponent.SetUpdatedComponent` (`self.RotatingMovement`) (`self.StaticMesh`)))

(event `self.ProjectileMovement.OnProjectileStop`
  (params (ImpactResult :type "HitResult Structure (by ref)"))
  (bind (_bblockinghit _binitialoverlap _time _distance _location _impactpoint _normal _impactnormal _physmat _hitactor _hitcomponent _hitbonename _bonename _hititem _elementindex _faceindex _tracestart) (`GameplayStatics.BreakHitResult` ImpactResult))
  (`GameplayStatics.ApplyPointDamage` _hitactor (`self.Damage`) _tracestart ImpactResult null self)
  (`self.K2_DestroyActor`)
  (cast `/Game/Blueprints/BP_Ship` _hitactor)
  (`GameplayStatics.SpawnEmitterAtLocation` "/Game/InfinityBladeEffects/Effects/FX_Mobile/combat/P_Impact_Golem_Gib_Fire.P_Impact_Golem_Gib_Fire" _impactpoint (struct) (`KismetMathLibrary.MakeVector` 1.0 1.0 1.0)))

(fn `UserConstructionScript`)