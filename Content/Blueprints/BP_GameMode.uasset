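; Game mode Blueprint that binds an enemy spawn handler and initializes the map on BeginPlay.
; The SpawnEnemy handler currently only prints the received enemy death tag.
; Disconnected nodes hold logic to spawn BP_Ship at an offset random navigable point around the player and set its death tag, but none of it runs.
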(event `self.ReceiveBeginPlay`
  (`KismetSystemLibrary.PrintString` "Binding spawn event")
  (add `self.OnSpawnEnemy` (delegate `SpawnEnemy`))
  (`self.InitializeMap`))

(event `SpawnEnemy` :!signature `self.OnSpawnEnemy`
  (params (EnemyDeathTag :type "GameplayTag Structure"))
  (`KismetSystemLibrary.PrintString` (`KismetStringLibrary.Conv_NameToString` (`BlueprintGameplayTagLibrary.GetTagName` EnemyDeathTag))))

(fn `UserConstructionScript`)