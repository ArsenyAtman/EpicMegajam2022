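; BP_EnemyAIC is an enemy AI controller that runs a default behavior tree on BeginPlay and tracks the player's ship through AI perception.
; When a perception update includes the player pawn, it casts that pawn to BP_Ship, stores it as Player and prints a debug message.
; A valid Player reference is cleared whenever an update omits it, with no check of whether the stimulus was sensed or lost.
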(event `self.ReceiveBeginPlay`
  (`self.RunBehaviorTree` (`BehaviorTreeComponent.DefaultBehaviorTreeAsset` (`self.BehaviorTree`))))

(event `self.AIPerception.OnPerceptionUpdated`
  (params (UpdatedActors :type "Array of Actor Object Reference (by ref)"))
  (bind _returnvalue (`KismetArrayLibrary.Array_Find` UpdatedActors (`GameplayStatics.GetPlayerPawn` 0)))
  (if (and (`KismetSystemLibrary.IsValid` (`self.Player`)) (not (`KismetArrayLibrary.Array_Contains` UpdatedActors (`self.Player`))))
    (set `self.Player` null)
    (elif (`KismetArrayLibrary.Array_IsValidIndex` UpdatedActors _returnvalue)
      (bind _asbp_ship (cast `/Game/Blueprints/BP_Ship` (`|GetArrayItem` UpdatedActors _returnvalue)))
      (set `self.Player` _asbp_ship)
      (if true
        (`KismetSystemLibrary.PrintString` "Hello")))))

(fn `UserConstructionScript`)