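; Cannon actor that fires BP_CannonBall projectiles on request, gated by a cooldown.
; Fire waits a random delay, then starts the timer-based cooldown and plays the Recoil timeline.
; The timeline slides the cannon along its local Y axis, and its Fire event track spawns the ball at the Arrow component.
; Launch direction is randomized within a Spread-angle cone around the Arrow's forward vector.
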(event `Fire`
  (bind _arrow (`self.Arrow`))
  (if (`self.CanFire`)
    (`KismetSystemLibrary.Delay` (`KismetMathLibrary.RandomFloatInRange` (`self.MinFireDelay`) (`self.MaxFireDelay`)))
    (`self.CooldownStart`)
    (bind (_direction _recoil) (`Timeline|Recoil` :!via `PlayFromStart`)
      (:`Update`
        (`SceneComponent.K2_SetRelativeLocation` (`self.Cannon`) (`KismetMathLibrary.MakeVector` 0.0 _recoil) false false))
      (:`Fire`
        (`|SpawnActorFromClass` "/Game/Blueprints/BP_CannonBall.BP_CannonBall_C" (`KismetMathLibrary.MakeTransform` (`SceneComponent.K2_GetComponentLocation` _arrow) (`KismetMathLibrary.MakeRotFromX` (`KismetMathLibrary.RandomUnitVectorInConeInDegrees` (`SceneComponent.GetForwardVector` _arrow) (`self.Spread`)))) "Undefined" "OverrideRootScale" null null)))))

(event `CooldownStart`
  (set `self.CanFire` false)
  (`KismetSystemLibrary.K2_SetTimerDelegate` (delegate `CooldownEnd`) (`self.CooldownTime`)))

(event `CooldownEnd`
  (set `self.CanFire` true))

(fn `UserConstructionScript`)