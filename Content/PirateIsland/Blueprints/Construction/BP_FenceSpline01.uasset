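; Construction-script fence builder that lays copies of a static mesh along a spline and snaps them to the ground.
; It adds one mesh component per spline segment, at a fixed scale, rotated to look at the next point rather than deformed.
; Each point is traced downward for the ground and given a random height offset, and each mesh gets a random roll for an uneven look.
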(fn `F_GetGroundLocation`
  (params (SplinePointLocation :type "Vector Structure"))
  (returns (GroundLocation :type "Vector Structure"))
  (bind _outhit (`KismetSystemLibrary.LineTraceSingle` SplinePointLocation (- SplinePointLocation (0.0 0.0 1000.0)) "TraceTypeQuery1" true))
  (return (+ (`.Location` (`GameplayStatics.BreakHitResult` _outhit)) (`KismetMathLibrary.MakeVector` 0.0 0.0 (`KismetMathLibrary.RandomFloatInRange` (`self.ZOffsetMin`) (`self.ZOffsetMax`))))))

(fn `UserConstructionScript`
  (locals (CurrentMesh :type "StaticMeshComponent Object Reference") (CurrentGroundLocation :type "Vector Structure") (NextGroundLocation :type "Vector Structure" :default (0.0 0.0 0.0)))
  (for _index (range (+ (- (`SplineComponent.GetNumberOfSplinePoints` (`self.Spline`)) 2) 1))
    (bind _returnvalue (`AddComponent|NODE_AddStaticMeshComponent-0`))
    (bind _output_get (set `local.CurrentMesh` _returnvalue))
    (`StaticMeshComponent.SetStaticMesh` _output_get (`self.Mesh`))
    (bind _groundlocation (`self.F_GetGroundLocation` (`SplineComponent.GetLocationAtSplinePoint` (`self.Spline`) _index "World")))
    (set `local.CurrentGroundLocation` _groundlocation)
    (bind _groundlocation_2 (`self.F_GetGroundLocation` (`SplineComponent.GetLocationAtSplinePoint` (`self.Spline`) (+ 1 _index) "World")))
    (set `local.NextGroundLocation` _groundlocation_2)
    (`SceneComponent.K2_SetWorldTransform` (`local.CurrentMesh`) (`KismetMathLibrary.MakeTransform` (`local.CurrentGroundLocation`) (`KismetMathLibrary.FindLookAtRotation` (`local.CurrentGroundLocation`) (`local.NextGroundLocation`)) (`self.Scale`)) false false)
    (`SceneComponent.K2_AddLocalRotation` (`local.CurrentMesh`) (`KismetMathLibrary.MakeRotator` (`KismetMathLibrary.RandomFloatInRange` (`self.RollMin`) (`self.RollMax`))) false false)))