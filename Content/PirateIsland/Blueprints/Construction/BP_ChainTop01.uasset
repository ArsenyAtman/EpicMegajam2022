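; BP_ChainTop01 is a construction-time Blueprint that builds a chain hanging downward from the actor's origin.
; The construction script divides the length by the link spacing and adds one static mesh component per link, stepping down local Z.
; A FlipFlop alternates each link's base yaw by a quarter turn, with an extra per-link twist from RotateAlong.
; The event graph holds only disabled placeholder events, so it adds no runtime logic.
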(fn `UserConstructionScript`
  (locals (Count :type Integer) (Yaw :type "Float (double-precision)"))
  (set `local.Count` (`KismetMathLibrary.FTrunc` (/ (`self.Lenght`) (`self.DistanceBetween`))))
  (for _index (range (+ (`local.Count`) 1))
    (`/Engine/EditorBlueprintResources/StandardMacros.FlipFlop`
      (:`A`
        (bind _returnvalue (* _index (`self.RotateAlong`)))
        (set `local.Yaw` (+ 0.0 _returnvalue)))
      (:`B`
        (set `local.Yaw` (+ 90.0 _returnvalue))))
    (`AddComponent|NODE_AddStaticMeshComponent-0` :`RelativeTransform` (`KismetMathLibrary.MakeTransform` (`KismetMathLibrary.MakeVector` 0.0 0.0 (* (+ (* _index (`self.DistanceBetween`)) 9.0) -1.0)) (`KismetMathLibrary.MakeRotator` 0.0 90.0 (`local.Yaw`))))))